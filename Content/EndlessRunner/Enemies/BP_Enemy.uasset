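; BP_Enemy is an endless-runner hazard that kills the player character on contact unless a shield is active.
; Its sphere overlap casts to BP_ThirdPersonCharacter and uses a BeenHit flag to react only once.
; A shielded hit teleports the enemy out of play below the world origin instead of destroying it, then breaks the shield.
; An unshielded hit prints the score, Points plus the player's X position, and destroys the player.
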(event `self.Sphere.OnComponentBeginOverlap`
  (params (OverlappedComponent :type "PrimitiveComponent Object Reference") (OtherActor :type "Actor Object Reference") (OtherComp :type "PrimitiveComponent Object Reference") (OtherBodyIndex :type Integer) (bFromSweep :type Boolean) (SweepResult :type "HitResult Structure (by ref)"))
  (bind _asbp_third_person_character (cast `/Game/ThirdPerson/Blueprints/BP_ThirdPersonCharacter` OtherActor))
  (if (not (`self.BeenHit`))
    (set `self.BeenHit` true)
    (if (`/Game/ThirdPerson/Blueprints/BP_ThirdPersonCharacter.Shielded` _asbp_third_person_character)
      (`self.K2_SetActorLocation` (0.0 0.0 -1000.0))
      (`/Game/ThirdPerson/Blueprints/BP_ThirdPersonCharacter.ShieldBreak` _asbp_third_person_character)
      (else
        (`KismetSystemLibrary.PrintString` (`KismetStringLibrary.Conv_DoubleToString` (+ (`/Game/ThirdPerson/Blueprints/BP_ThirdPersonCharacter.Points` _asbp_third_person_character) (.x (`self.K2_GetActorLocation` _asbp_third_person_character)))))
        (`self.K2_DestroyActor` _asbp_third_person_character)))))

(fn `UserConstructionScript`)