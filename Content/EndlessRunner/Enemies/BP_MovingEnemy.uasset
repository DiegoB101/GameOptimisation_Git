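; BP_MovingEnemy is an endless runner enemy that slides back and forth along world Y and notifies whatever actor hits it.
; A looping timer drives a FlipFlop that plays or reverses a Timeline, lerping between the endpoints set by SetMovement.
; The first sphere overlap sends PlayerHitMessage, drops the enemy below the world and re-bases its path at the origin.
; Reset only clears the BeenHit guard.
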(event `self.ReceiveBeginPlay`
  (`|ExecutionSequence`
    (:`then_0`
      (`self.SetMovement` (`self.K2_GetActorLocation`)))
    (:`then_1`
      (`KismetSystemLibrary.K2_SetTimerDelegate` (delegate `Move`) 1.0 true))))

(event `self.Sphere.OnComponentBeginOverlap`
  (params (OverlappedComponent :type "PrimitiveComponent Object Reference") (OtherActor :type "Actor Object Reference") (OtherComp :type "PrimitiveComponent Object Reference") (OtherBodyIndex :type Integer) (bFromSweep :type Boolean) (SweepResult :type "HitResult Structure (by ref)"))
  (if (not (`self.Been Hit`))
    (set `self.Been Hit` true)
    (message `/Game/EndlessRunner/Enemies/I_PlayerHit.PlayerHit` OtherActor null)
    (`self.K2_SetActorLocation` (0.0 0.0 -1000.0))
    (`self.SetMovement` (0.0 0.0 0.0))))

(event `Move`
  (`/Engine/EditorBlueprintResources/StandardMacros.FlipFlop`
    (:`A`
      (bind (_direction _newtrack_0) (`Timeline|Timeline` :!label _label)
        (:`Update`
          (`self.K2_SetActorLocation` (`KismetMathLibrary.VLerp` (`self.Start Location`) (`self.End Location`) _newtrack_0)))))
    (:`B`
      (goto _label :!via `Reverse`))))

(event `/Game/EndlessRunner/I_Reset.Reset`
  (set `self.Been Hit` false))

(fn `SetMovement`
  (params (`New Location` :type "Vector Structure"))
  (bind _output_get (set `self.Start Location` `New Location`))
  (set `self.End Location` (`KismetMathLibrary.MakeVector` (.x _output_get) (+ (.y _output_get) 300.0) (.z _output_get))))

(fn `UserConstructionScript`)