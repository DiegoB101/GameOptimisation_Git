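; Endless runner level constructor that lays out pickups and enemies ahead of the player by repositioning actors already in the level.
; BeginPlay gathers pickup, static and moving enemy pools, takes the GameInstance seed and places Pattern1 twice, 1000 units apart.
; Reset re-anchors to the player's X, then GenerateObstacles picks among ten lane-based patterns using the seeded random stream.
; Only Pattern1 moves placed actors out of their pool into UsedActors.
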(event `self.ReceiveBeginPlay`
  (`self.SetLocation`)
  (bind _outactors (`GameplayStatics.GetAllActorsOfClass` "/Game/EndlessRunner/Pickups/B_PickupMaster.B_PickupMaster_C"))
  (for _array_element _outactors
    (`KismetArrayLibrary.Array_Add` (`self.AllPickups`) _array_element))
  (bind _outactors_2 (`GameplayStatics.GetAllActorsOfClass` "/Game/EndlessRunner/Enemies/BP_Enemystatic.BP_Enemystatic_C"))
  (for _array_element_2 _outactors_2
    (`KismetArrayLibrary.Array_Add` (`self.AllStaticEnemies`) _array_element_2))
  (bind _outactors_3 (`GameplayStatics.GetAllActorsOfClass` "/Game/EndlessRunner/Enemies/BP_MovingEnemy.BP_MovingEnemy_C"))
  (for _array_element_3 _outactors_3
    (`KismetArrayLibrary.Array_Add` (`self.AllMovingEnemies`) _array_element_3))
  (bind _asmain_game_instance (cast `/Game/EndlessRunner/MainGameInstance` (`GameplayStatics.GetGameInstance`)))
  (set `self.SeedReference` (`/Game/EndlessRunner/MainGameInstance.Seed` _asmain_game_instance))
  (`self.Pattern 1`)
  (set `self.ConstructorLocation` (+ (`self.ConstructorLocation`) (1000.0 0.0 0.0)))
  (`self.Pattern 1`))

(event `/Game/EndlessRunner/I_Reset.Reset`
  (`self.SetLocation`)
  (`self.GenerateObstacles`))

(fn `ActorIsUsed`
  (params (UsedActor :type "Actor Object Reference") (UsedArray :type "Array of Actor Object Reference") (UsedIndex :type Integer))
  (`KismetArrayLibrary.Array_Remove` UsedArray UsedIndex)
  (`KismetArrayLibrary.Array_Add` (`self.UsedActors`) UsedActor))

(fn `GenerateObstacles`
  (switch `int` (`KismetMathLibrary.RandomIntegerFromStream` (`self.SeedReference`) 10)
    (:`1`
      (`self.Pattern 1`))
    (:`2`
      (`self.Pattern 2`))
    (:`3`
      (`self.Pattern 3`))
    (:`4`
      (`self.Pattern 4`))
    (:`5`
      (`self.Pattern 5`))
    (:`6`
      (`self.Pattern 6`))
    (:`7`
      (`self.Pattern 7`))
    (:`8`
      (`self.Pattern 8`))
    (:`9`
      (`self.pattern 9`))
    (:`10`
      (`self.pattern 10`))))

(fn `Pattern 1`
  (locals (pointsCounter :type Integer) (shieldCounter :type Integer))
  (bind _allpickups (`self.AllPickups`))
  (for (_array_element _array_index) _allpickups
    (bind _returnvalue (`GameplayStatics.GetObjectClass` _array_element))
    (if (== _returnvalue "/Game/EndlessRunner/Pickups/B_PointsPickup.B_PointsPickup_C")
      (bind _output_get (set `local.pointsCounter` (+ (`local.pointsCounter`) 1)))
      (switch `int` _output_get
        (:`1`
          (`self.PlaceActor` 500 -200 _array_element)
          (`self.ActorIsUsed` _array_element _allpickups _array_index))
        (:`2`
          (`self.PlaceActor` 500 200 _array_element)
          (`self.ActorIsUsed` _array_element _allpickups _array_index)))
      (elif (== _returnvalue "/Game/EndlessRunner/Pickups/B_ShieldPickup.B_ShieldPickup_C")
        (bind _output_get_2 (set `local.shieldCounter` (+ (`local.shieldCounter`) 1)))
        (switch `int` _output_get_2
          (:`1`
            (`self.PlaceActor` 500 0 _array_element)
            (`self.ActorIsUsed` _array_element _allpickups _array_index)))))))

(fn `pattern 10`
  (locals (Pointscounter :type Integer))
  (bind _allpickups (`self.AllPickups`))
  (for _array_element _allpickups
    (if (== (`GameplayStatics.GetObjectClass` _array_element) "/Game/EndlessRunner/Pickups/B_SpeedPickup.B_SpeedPickup_C")
      (`self.PlaceActor` 500 200 _array_element)
      (break)))
  (for _array_element_2 _allpickups
    (if (== (`GameplayStatics.GetObjectClass` _array_element_2) "/Game/EndlessRunner/Pickups/B_PointsPickup.B_PointsPickup_C")
      (bind _result (`/Engine/EditorBlueprintResources/StandardMacros.IncrementInt` (`local.Pointscounter`))
        (:`  `
          (switch `int` _result
            (:`1`
              (`self.PlaceActor` 800 0 _array_element_2))
            (:`2`
              (`self.PlaceActor` 1100 0 _array_element_2))
            (:`3`
              (`self.PlaceActor` 1400 0 _array_element_2))
            (:`4`
              (`self.PlaceActor` 1400 -200 _array_element_2))
            (:`5`
              (`self.PlaceActor` 1700 -200 _array_element_2))))))))

(fn `Pattern 2`
  (locals (PointsCounter :type Integer))
  (for _array_element (`self.AllPickups`)
    (if (== (`GameplayStatics.GetObjectClass` _array_element) "/Game/EndlessRunner/Pickups/B_PointsPickup.B_PointsPickup_C")
      (set `local.PointsCounter` (+ (`local.PointsCounter`) 1))
      (switch `int` (`local.PointsCounter`)
        (:`1`
          (`self.PlaceActor` 500 -200 _array_element))
        (:`2`
          (`self.PlaceActor` 800 -200 _array_element))
        (:`3`
          (`self.PlaceActor` 1100 -200 _array_element))))))

(fn `Pattern 3`
  (locals (PointsCounter :type Integer))
  (for _array_element (`self.AllPickups`)
    (if (== (`GameplayStatics.GetObjectClass` _array_element) "/Game/EndlessRunner/Pickups/B_PointsPickup.B_PointsPickup_C")
      (set `local.PointsCounter` (+ (`local.PointsCounter`) 1))
      (switch `int` (`local.PointsCounter`)
        (:`1`
          (`self.PlaceActor` 500 200 _array_element))
        (:`2`
          (`self.PlaceActor` 800 200 _array_element))
        (:`3`
          (`self.PlaceActor` 1100 200 _array_element))))))

(fn `Pattern 4`
  (locals (EnemyCounter :type Integer) (pointsCounter :type Integer))
  (for _array_element (`self.AllStaticEnemies`)
    (bind _output_get (set `local.EnemyCounter` (+ (`local.EnemyCounter`) 1)))
    (switch `int` _output_get
      (:`1`
        (`self.PlaceActor` 800 0 _array_element))
      (:`2`
        (`self.PlaceActor` 800 -200 _array_element)
        (break))))
  (for _array_element_2 (`self.AllPickups`)
    (bind _output_get_2 (set `local.pointsCounter` (+ (`local.pointsCounter`) 1)))
    (if (== (`GameplayStatics.GetObjectClass` _array_element_2) "/Game/EndlessRunner/Pickups/B_PointsPickup.B_PointsPickup_C")
      (switch `int` _output_get_2
        (:`1`
          (`self.PlaceActor` 500 200 _array_element_2))
        (:`2`
          (`self.PlaceActor` 800 200 _array_element_2))
        (:`3`
          (`self.PlaceActor` 1100 200 _array_element_2))))))

(fn `Pattern 5`
  (locals (PointsCounter :type Integer) (EnemyCounter :type Integer))
  (for _array_element (`self.AllStaticEnemies`)
    (bind _output_get (set `local.EnemyCounter` (+ (`local.EnemyCounter`) 1)))
    (switch `int` _output_get
      (:`1`
        (`self.PlaceActor` 800 0 _array_element))
      (:`2`
        (`self.PlaceActor` 800 200 _array_element)
        (break))))
  (for _array_element_2 (`self.AllPickups`)
    (bind _output_get_2 (set `local.pointsCounter` (+ (`local.pointsCounter`) 1)))
    (if (== (`GameplayStatics.GetObjectClass` _array_element_2) "/Game/EndlessRunner/Pickups/B_PointsPickup.B_PointsPickup_C")
      (switch `int` _output_get_2
        (:`1`
          (`self.PlaceActor` 500 -200 _array_element_2))
        (:`2`
          (`self.PlaceActor` 800 -200 _array_element_2))
        (:`3`
          (`self.PlaceActor` 1100 -200 _array_element_2))))))

(fn `Pattern 6`
  (locals (PointsCounter :type Integer) (EnemyCounter :type Integer))
  (for _array_element (`self.AllStaticEnemies`)
    (bind _output_get (set `local.EnemyCounter` (+ (`local.EnemyCounter`) 1)))
    (switch `int` _output_get
      (:`1`
        (`self.PlaceActor` 800 200 _array_element))
      (:`2`
        (`self.PlaceActor` 800 -200 _array_element)
        (break))))
  (for _array_element_2 (`self.AllPickups`)
    (bind _output_get_2 (set `local.pointsCounter` (+ (`local.pointsCounter`) 1)))
    (if (== (`GameplayStatics.GetObjectClass` _array_element_2) "/Game/EndlessRunner/Pickups/B_PointsPickup.B_PointsPickup_C")
      (switch `int` _output_get_2
        (:`1`
          (`self.PlaceActor` 500 0 _array_element_2))
        (:`2`
          (`self.PlaceActor` 800 0 _array_element_2))
        (:`3`
          (`self.PlaceActor` 1100 0 _array_element_2))))))

(fn `Pattern 7`
  (locals (PointsCounter :type Integer))
  (for _array_element (`self.AllPickups`)
    (bind _returnvalue (`GameplayStatics.GetObjectClass` _array_element))
    (if (== _returnvalue "/Game/EndlessRunner/Pickups/B_PointsPickup.B_PointsPickup_C")
      (bind _output_get (set `local.PointsCounter` (+ (`local.PointsCounter`) 1)))
      (switch `int` _output_get
        (:`1`
          (`self.PlaceActor` 800 0 _array_element))
        (:`2`
          (`self.PlaceActor` 800 200 _array_element))
        (:`3`
          (`self.PlaceActor` 800 -200 _array_element)))
      (elif (== _returnvalue "/Game/EndlessRunner/Pickups/B_ShieldPickup.B_ShieldPickup_C")
        (`self.PlaceActor` 500 0 _array_element))))
  (for _array_element_2 (`self.AllMovingEnemies`)
    (`self.PlaceMovingEnemy` 1100.0 -200.0 1100.0 200.0 _array_element_2)
    (break)))

(fn `Pattern 8`
  (locals (MoverCounter :type Integer))
  (for _array_element (`self.AllMovingEnemies`)
    (bind _result (`/Engine/EditorBlueprintResources/StandardMacros.IncrementInt` (`local.MoverCounter`))
      (:`  `
        (switch `int` _result
          (:`1`
            (`self.PlaceMovingEnemy` 500.0 200.0 500.0 -200.0 _array_element))
          (:`2`
            (`self.PlaceMovingEnemy` 1500.0 -200.0 1500.0 200.0 _array_element)
            (break))))))
  (for _array_element_2 (`self.AllPickups`)
    (if (== (`GameplayStatics.GetObjectClass` _array_element_2) "/Game/EndlessRunner/Pickups/B_ShieldPickup.B_ShieldPickup_C")
      (`self.PlaceActor` 1100 0 _array_element_2))))

(fn `pattern 9`
  (locals (Pointscounter :type Integer))
  (bind _allpickups (`self.AllPickups`))
  (for _array_element _allpickups
    (if (== (`GameplayStatics.GetObjectClass` _array_element) "/Game/EndlessRunner/Pickups/B_SpeedPickup.B_SpeedPickup_C")
      (`self.PlaceActor` 500 -200 _array_element)
      (break)))
  (for _array_element_2 _allpickups
    (if (== (`GameplayStatics.GetObjectClass` _array_element_2) "/Game/EndlessRunner/Pickups/B_PointsPickup.B_PointsPickup_C")
      (bind _result (`/Engine/EditorBlueprintResources/StandardMacros.IncrementInt` (`local.Pointscounter`))
        (:`  `
          (switch `int` _result
            (:`1`
              (`self.PlaceActor` 800 0 _array_element_2))
            (:`2`
              (`self.PlaceActor` 1100 0 _array_element_2))
            (:`3`
              (`self.PlaceActor` 1400 0 _array_element_2))
            (:`4`
              (`self.PlaceActor` 1400 200 _array_element_2))
            (:`5`
              (`self.PlaceActor` 1700 200 _array_element_2))))))))

(fn `PlaceActor`
  (params (Xoffset :type Integer) (Yoffset :type Integer) (Actor :type "Actor Object Reference"))
  (`self.K2_SetActorLocation` Actor (`KismetMathLibrary.MakeVector` (+ (.x (`self.ConstructorLocation`)) Xoffset) (+ (.y (`self.ConstructorLocation`)) Yoffset) (.z (`self.ConstructorLocation`))) false false))

(fn `PlaceMovingEnemy`
  (params (StarX :type "Float (double-precision)") (StartY :type "Float (double-precision)") (EndX :type "Float (double-precision)") (EnxY :type "Float (double-precision)") (Mover :type "/Game/EndlessRunner/Enemies/BP_MovingEnemy Object Reference"))
  (locals (Direction :type Integer))
  (bind _returnvalue (`KismetMathLibrary.MakeVector` (+ (.x (`self.ConstructorLocation`)) StarX) (+ (.y (`self.ConstructorLocation`)) StartY) (.z (`self.ConstructorLocation`))))
  (set `/Game/EndlessRunner/Enemies/BP_MovingEnemy.Start Location` _returnvalue Mover)
  (set `/Game/EndlessRunner/Enemies/BP_MovingEnemy.End Location` (`KismetMathLibrary.MakeVector` (+ (.x (`self.ConstructorLocation`)) EndX) (+ (.y (`self.ConstructorLocation`)) EnxY) (.z (`self.ConstructorLocation`))) Mover)
  (`self.K2_SetActorLocation` Mover _returnvalue false false))

(fn `SetLocation`
  (bind _output_get (set `self.ConstructorLocation` (`KismetMathLibrary.MakeVector` (+ (.x (`self.K2_GetActorLocation` (`GameplayStatics.GetPlayerCharacter` 0))) 200.0) 0.0 (.z (`self.K2_GetActorLocation` (`GameplayStatics.GetPlayerCharacter` 0))))))
  (`self.K2_SetActorLocation` _output_get))

(fn `UserConstructionScript`)